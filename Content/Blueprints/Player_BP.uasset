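; Side-scrolling flipbook player character that waters trees, feeds them photons and catches worms (Minhoca).
; Input picks one of three tools; the action freezes movement and applies it to the target found by the ColisaoFerramentas overlap, spending water or photons collected through capsule overlaps.
; Tick updates facing and animation and calls Derrota when lives run out from damage.
; Derrota and Vitoria stop the Spawner and show end screens.
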(event OnComponentBeginOverlap(CapsuleComponent)
  (params (OverlappedComponent :type Primitive%20Component%20Object%20Reference) (OtherActor :type Actor%20Object%20Reference) (OtherComp :type Primitive%20Component%20Object%20Reference) (OtherBodyIndex :type Integer) (bFromSweep :type Boolean) (SweepResult :type Hit%20Result%20Structure%20%28by%20ref%29))
  (if (and (Actor|ActorHasTag OtherActor "agua") (<= (Variables|Default|Getagua) 20))
    (Variables|Default|Setagua (+ (Variables|Default|Getagua) 1))
    (Audio|PlaySound2D "/Game/Sounds/fx/gather.gather" 1.0 1.0 0.0 0 0 :!label _label)
    (Actor|DestroyActor OtherActor)
    (elif (and (Actor|ActorHasTag OtherActor "foton") (<= (Variables|Default|Getfoton) 20))
      (Variables|Default|Setfoton (+ (Variables|Default|Getfoton) 1))
      (goto _label))))

(event OnComponentEndOverlap(ColisaoFerramentas)
  (params (OverlappedComponent :type Primitive%20Component%20Object%20Reference) (OtherActor :type Actor%20Object%20Reference) (OtherComp :type Primitive%20Component%20Object%20Reference) (OtherBodyIndex :type Integer))
  (Variables|Default|Setenemy 0))

(event OnComponentBeginOverlap(ColisaoFerramentas)
  (params (OverlappedComponent :type Primitive%20Component%20Object%20Reference) (OtherActor :type Actor%20Object%20Reference) (OtherComp :type Primitive%20Component%20Object%20Reference) (OtherBodyIndex :type Integer) (bFromSweep :type Boolean) (SweepResult :type Hit%20Result%20Structure%20%28by%20ref%29))
  (if (Actor|ActorHasTag OtherActor "minhoca")
    (bind _asminhoca (Utilities|Casting|CastToMinhoca OtherActor))
    (Variables|Default|Setenemy _asminhoca)
    (else
      (bind _asarvore (Utilities|Casting|CastToArvore OtherActor))
      (Variables|Default|SetarvoreTarget _asarvore))))

(event Custom|UpdateRotation
  (Utilities|IsValid (Pawn|GetController)
    (:Is%20Valid
      (Math|Float|CompareFloat 0.0 (.x (Variables|/Script/Engine.MovementComponent|GetVelocity (Variables|Character|GetCharacterMovement)))
        (:>
          (Pawn|SetControlRotation (Pawn|GetController) (Math|Rotator|MakeRotator 0.0 0.0 1.8e+02)))
        (:<
          (Pawn|SetControlRotation (Pawn|GetController) (Math|Rotator|MakeRotator 0.0 0.0 0.0)))))))

(event Custom|ToolsAction
  (bind _arvoretarget (Variables|Default|GetarvoreTarget))
  (bind _arvoretarget_2 (Variables|Default|GetarvoreTarget))
  (bind _enemy (Variables|Default|Getenemy))
  (switch int (Variables|Default|Gettool)
    (:0
      (Utilities|IsValid _arvoretarget_2
        (:Is%20Valid
          (if (> (Variables|Default|Getagua) 0)
            (Variables|/Game/Blueprints/Arvore.Arvore_C|Setwater _arvoretarget (Math|Float|Clamp(Float) (+ (Variables|/Game/Blueprints/Arvore.Arvore_C|Getwater _arvoretarget) (Variables|Default|GettaxRecover)) 0.0 (Variables|/Game/Blueprints/Arvore.Arvore_C|GetwaterLevel _arvoretarget)))
            (bind _result (Math|Integer|DecrementInt (Variables|Default|Getagua))
              (:%20%20
                (Variables|Default|Setagua _result)
                (Audio|PlaySound2D "/Game/Sounds/fx/Jump9.Jump9" 1.0 1.0 0.0 0 0 :!label _label)))))))
    (:1
      (Utilities|IsValid _arvoretarget_2
        (:Is%20Valid
          (if (> (Variables|Default|Getfoton) 0)
            (Variables|/Game/Blueprints/Arvore.Arvore_C|Setfoton _arvoretarget (Math|Float|Clamp(Float) (+ (Variables|/Game/Blueprints/Arvore.Arvore_C|Getfoton _arvoretarget) (Variables|Default|GettaxRecover)) 0.0 (Variables|/Game/Blueprints/Arvore.Arvore_C|GetfotonLevel _arvoretarget)))
            (bind _result_2 (Math|Integer|DecrementInt (Variables|Default|Getfoton))
              (:%20%20
                (Variables|Default|Setfoton _result_2)
                (goto _label)))))))
    (:2
      (Utilities|IsValid _enemy
        (:Is%20Valid
          (Actor|DestroyActor _enemy)
          (Audio|PlaySound2D "/Game/Sounds/fx/Powerup6.Powerup6" 1.0 1.0 0.0 0 0))))))

(event Custom|UpdateAnimation
  (if (Variables|Default|GetinAction)
    (Sprite|SetFlipbook (Variables|Default|GetSprite) (Utilities|Select :Index (Variables|Default|Gettool) :Option%200 "/Game/Sprites/Personagem/personagem_regando.personagem_regando" :Option%201 "/Game/Sprites/Personagem/Foton_action_Flipbook.Foton_action_Flipbook" :Option%202 "/Game/Sprites/Personagem/captura.captura"))
    (else
      (Sprite|SetFlipbook (Variables|Default|GetSprite) (select (> (Math|Vector|VectorLength (Variables|/Script/Engine.MovementComponent|GetVelocity (Variables|Character|GetCharacterMovement))) 0.0) "/Game/Sprites/Personagem/Idle_move/personagem_walk.personagem_walk" "/Game/Sprites/Personagem/Idle_move/personagem_idle.personagem_idle")))))

(event Custom|Derrota
  (Variables|Default|Setderrotado true)
  (Variables|/Game/Blueprints/Spawner.Spawner_C|Setactive (Variables|Default|Getspawn) false)
  (bind _returnvalue (UserInterface|CreateWidget "/Game/UI/GameOver.GameOver_C"))
  (UserInterface|Viewport|AddtoViewport _returnvalue 0))

(event Custom|Vitoria
  (Variables|Default|Setderrotado true)
  (Variables|/Game/Blueprints/Spawner.Spawner_C|Setactive (Variables|Default|Getspawn) false)
  (bind _returnvalue (UserInterface|CreateWidget "/Game/UI/WIn.WIn_C"))
  (UserInterface|Viewport|AddtoViewport _returnvalue 0))

(event EventTick
  (params (DeltaSeconds :type Float%20%28single-precision%29))
  (CallFunction|UpdateRotation)
  (CallFunction|UpdateAnimation)
  (if (not (> (Variables|Default|Getvidas) 0))
    (CallFunction|Derrota)))

(event EventBeginPlay
  (bind _returnvalue (Game|GetPlayerController 0))
  (bind _returnvalue_2 (UserInterface|CreateWidget "/Game/UI/HUD.HUD_C"))
  (bind _output_get (Variables|Default|SetHUDRef _returnvalue_2))
  (UserInterface|Viewport|AddtoViewport _output_get 0)
  (Variables|/Script/Engine.PlayerController|SetbShowMouseCursor _returnvalue false)
  (Input|SetInputModeGameOnly _returnvalue false)
  (bind _returnvalue_3 (Actor|GetActorOfClass "/Game/Blueprints/Spawner.Spawner_C"))
  (Variables|Default|Setspawn _returnvalue_3))

(event Game|Damage|EventAnyDamage
  (params (Damage :type Float%20%28single-precision%29) (DamageType :type Damage%20Type%20Object%20Reference) (InstigatedBy :type Controller%20Object%20Reference) (DamageCauser :type Actor%20Object%20Reference))
  (Variables|Default|Setvidas (Math|Float|Truncate (- (Variables|Default|Getvidas) Damage))))

(event Input|ActionEvents|InputActionREgador
  (params (Key :type Key%20Structure :default "None"))
  (:Pressed
    (Variables|Default|Settool 0)
    (Default|UpdateHUDTools (Variables|Default|GetHUDRef))))

(event Input|ActionEvents|InputActionFoton
  (params (Key :type Key%20Structure :default "None"))
  (:Pressed
    (Variables|Default|Settool 1)
    (Default|UpdateHUDTools (Variables|Default|GetHUDRef))))

(event Input|ActionEvents|InputActionPegador
  (params (Key :type Key%20Structure :default "None"))
  (:Pressed
    (Variables|Default|Settool 2)
    (Default|UpdateHUDTools (Variables|Default|GetHUDRef))))

(event Input|ActionEvents|InputActionAcao
  (params (Key :type Key%20Structure :default "None"))
  (:Pressed
    (Variables|Default|SetinAction true)
    (CallFunction|ToolsAction)
    (Pawn|Components|CharacterMovement|SetMovementMode (Variables|Character|GetCharacterMovement) "MOVE_None" 0))
  (:Released
    (Variables|Default|SetinAction false)
    (Pawn|Components|CharacterMovement|SetMovementMode (Variables|Character|GetCharacterMovement) "MOVE_Walking" 0)))

(event Input|AxisEvents|InputAxisMoveHorizontal
  (params (AxisValue :type Float%20%28single-precision%29))
  (Pawn|Input|AddMovementInput "1.000000,0.000000,0.000000" AxisValue false))

(event Input|KeyboardEvents|Escape
  (params (Key :type Key%20Structure :default "None"))
  (:Pressed
    (Game|QuitGame (Game|GetPlayerController 0) "Quit" false)))

(fn ConstructionScript)