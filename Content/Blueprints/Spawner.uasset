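; Spawner actor that periodically drops either an Agua or a Foton actor into the level while Active is set.
; Tick accumulates time against a random interval between TimeMin and TimeMax, re-rolled after each spawn.
; Each spawn picks one of the two classes at random and places it at a random X position along a line with fixed Y and height.
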(event EventBeginPlay
  (Variables|Default|Settime%20respawn (Math|Random|RandomFloatinRange (Variables|Default|GettimeMin) (Variables|Default|GettimeMax))))

(event EventTick
  (params (DeltaSeconds :type Float%20%28single-precision%29))
  (if (Variables|Default|Getactive)
    (Variables|Default|Settime (+ (Variables|Default|Gettime) DeltaSeconds))
    (if (>= (Variables|Default|Gettime) (Variables|Default|Gettime%20respawn))
      (Game|SpawnActorfromClass (Utilities|Select :Index (Math|Random|RandomIntegerinRange 0 1) :Option%200 "/Game/Blueprints/Agua.Agua_C" :Option%201 "/Game/Blueprints/Foton.Foton_C") (Math|Transform|MakeTransform (Math|Vector|MakeVector (Math|Random|RandomFloatinRange 2e+02 2.4e+03) 29.0 1314.0) "0, 0, 0" "1.000000,1.000000,1.000000") "Undefined" 0 0)
      (Variables|Default|Settime 0.0)
      (Variables|Default|Settime%20respawn (Math|Random|RandomFloatinRange (Variables|Default|GettimeMin) (Variables|Default|GettimeMax))))))

(fn ConstructionScript)