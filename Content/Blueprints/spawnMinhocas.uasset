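; Spawner actor that repeatedly creates Minhoca (worm) actors at randomized intervals.
; Tick accumulates elapsed time until it reaches Timeload, then sets a Spawn flag that triggers the spawn on the following tick.
; Each spawn takes the spawner's X position with fixed Y and Z coordinates.
; RandomLoad picks a new delay between SpawntimeMin and SpawntimeMax at BeginPlay and before every spawn.
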(event Custom|RandomLoad
  (Variables|Default|Settimeload (Math|Random|RandomFloatinRange (Variables|Default|GetspawntimeMin) (Variables|Default|GetspawntimeMax))))

(event EventBeginPlay
  (CallFunction|RandomLoad))

(event EventTick
  (params (DeltaSeconds :type Float%20%28single-precision%29))
  (if (Variables|Default|Getspawn)
    (Variables|Default|Setspawn false)
    (CallFunction|RandomLoad)
    (Game|SpawnActorfromClass "/Game/Blueprints/Minhoca.Minhoca_C" (Math|Transform|MakeTransform (Math|Vector|MakeVector (.x (Transformation|GetActorLocation self)) 8.0 476.0) "0, 0, 0" "1.000000,1.000000,1.000000") "Undefined" 0 0)
    (else
      (Variables|Default|Settime (+ (Variables|Default|Gettime) DeltaSeconds))
      (if (>= (Variables|Default|Gettime) (Variables|Default|Gettimeload))
        (Variables|Default|Setspawn true)
        (Variables|Default|Settime 0.0)))))

(fn ConstructionScript)