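; Minhoca is an enemy character that drifts toward the player and damages it on contact.
; Each tick it interpolates its location toward player pawn 0 without sweeping and advances an attack cooldown timer.
; Capsule overlap with the cached Player_BP applies damage, plays a hit sound and resets the cooldown once the attack is ready.
; Control yaw flips on velocity length, so the 180-degree branch never fires.
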(event OnComponentBeginOverlap(CapsuleComponent)
  (params (OverlappedComponent :type Primitive%20Component%20Object%20Reference) (OtherActor :type Actor%20Object%20Reference) (OtherComp :type Primitive%20Component%20Object%20Reference) (OtherBodyIndex :type Integer) (bFromSweep :type Boolean) (SweepResult :type Hit%20Result%20Structure%20%28by%20ref%29))
  (bind _playerref (Variables|Default|GetPlayerREf))
  (if (== OtherComp (Variables|/Script/Engine.Character|GetCapsuleComponent _playerref))
    (if (Variables|Default|Getattack)
      (Game|Damage|ApplyDamage _playerref 1.0 0 0)
      (Audio|PlaySound2D "/Game/Sounds/fx/hit.hit" 1.0 1.0 0.0 0 0)
      (Variables|Default|Settime 0.0)
      (Variables|Default|Setattack false))))

(event Custom|UpdateRotation
  (bind _returnvalue (Pawn|GetController))
  (Math|Float|CompareFloat (Math|Vector|VectorLength (Variables|/Script/Engine.MovementComponent|GetVelocity (Variables|Character|GetCharacterMovement))) 0.0
    (:>
      (Pawn|SetControlRotation _returnvalue (Math|Rotator|MakeRotator 0.0 0.0 0.0)))
    (:<
      (Pawn|SetControlRotation _returnvalue (Math|Rotator|MakeRotator 0.0 0.0 1.8e+02)))))

(event Custom|PlayerFollow
  (params (delta :type Float%20%28double-precision%29))
  (Transformation|SetActorLocation (Math|Interpolation|VInterpTo (Transformation|GetActorLocation) (Transformation|GetActorLocation (Game|Player|GetPlayerPawn 0)) delta 0.4) false false))

(event Custom|LoadAttack
  (params (delta :type Float%20%28double-precision%29))
  (if (<= (Variables|Default|Gettime) (Variables|Default|Getload))
    (Variables|Default|Settime (+ (Variables|Default|Gettime) delta))
    (else
      (Variables|Default|Setattack true))))

(event EventBeginPlay
  (bind _returnvalue (Actor|GetActorOfClass "/Game/Blueprints/Player_BP.Player_BP_C"))
  (Variables|Default|SetPlayerREf _returnvalue))

(event EventTick
  (params (DeltaSeconds :type Float%20%28single-precision%29))
  (CallFunction|PlayerFollow DeltaSeconds)
  (CallFunction|LoadAttack DeltaSeconds)
  (CallFunction|UpdateRotation))

(fn ConstructionScript)