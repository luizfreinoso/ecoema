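; Tree actor that grows through five Paper2D flipbook stages and drives the game's win and loss.
; Tick drains water and photon levels, reporting defeat to the player when either empties, and advances growth on a timer.
; Each stage plays a transition flipbook, switches to that stage's flipbook after a delay, and raises the status widget.
; A fully grown tree updates the HUD message, then spawns another at a random free PosicaoPlanta or triggers victory.
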(event Custom|Evolucao
  (params (delta :type Float%20%28double-precision%29))
  (if (not (Variables|/Game/Blueprints/Player_BP.Player_BP_C|Getderrotado (Variables|Default|GetPlayerRef)))
    (bind _output_get (Variables|Default|Settime (+ delta (Variables|Default|Gettime))))
    (Variables|Default|Setwater (- (Variables|Default|Getwater) (* delta (Variables|Default|GettaxReaming))))
    (Variables|Default|Setfoton (- (Variables|Default|Getfoton) (* delta (Variables|Default|GettaxReaming))))
    (if (and (>= _output_get (Variables|Default|GettempoLevel)) (< (Variables|Default|Getlevel) 5))
      (Variables|Default|Settime 0.0)
      (Sprite|SetFlipbook (Variables|Default|GetPaperFlipbook) (Utilities|Select :Index (- (Variables|Default|Getlevel) 1) :Option%200 "/Game/Sprites/Arvore/FB/Arvore_FB2.Arvore_FB2" :Option%201 "/Game/Sprites/Arvore/FB/Arvore_FB3.Arvore_FB3" :Option%202 "/Game/Sprites/Arvore/FB/Arvore_FB4.Arvore_FB4" :Option%203 "/Game/Sprites/Arvore/FB/Arvore_FB5.Arvore_FB5"))
      (bind _result (Math|Integer|IncrementInt (Variables|Default|Getlevel))
        (:%20%20
          (Variables|Default|Setlevel _result)
          (CallFunction|UpdateUIPosition)
          (CallFunction|AnimacaoFim)
          (CallFunction|NovaArvore))))))

(event Custom|derrota
  (if (or (<= (Variables|Default|Getwater) 0.0) (<= (Variables|Default|Getfoton) 0.0))
    (Default|Derrota (Variables|Default|GetPlayerRef))))

(event Custom|AnimacaoFim
  (Utilities|FlowControl|Delay (Class|PaperFlipbookComponent|GetFlipbookLength (Variables|Default|GetPaperFlipbook)))
  (Sprite|SetFlipbook (Variables|Default|GetPaperFlipbook) (Utilities|Select :Index (- (Variables|Default|Getlevel) 1) :Option%200 "/Game/Sprites/Arvore/FB/Arvore_muda.Arvore_muda" :Option%201 "/Game/Sprites/Arvore/FB/Arvore_muda_2.Arvore_muda_2" :Option%202 "/Game/Sprites/Arvore/FB/Arvore_muda_3.Arvore_muda_3" :Option%203 "/Game/Sprites/Arvore/FB/Arvore_muda_4.Arvore_muda_4" :Option%204 "/Game/Sprites/Arvore/FB/Arvore_muda_5.Arvore_muda_5")))

(event Custom|NovaArvore
  (if (>= (Variables|Default|Getlevel) 5)
    (CallFunction|MensagensUsuario)
    (if (< (Variables|Default|GetNumTreesAux) 2)
      (bind _outactors (Actor|GetAllActorsOfClass "/Game/Blueprints/PosicaoPlanta.PosicaoPlanta_C"))
      (Utilities|Array|Shuffle _outactors)
      (bind _array_element (Utilities|Array|ForEachLoopwithBreak _outactors :!label _label)
        (:LoopBody
          (if (not (Variables|/Game/Blueprints/PosicaoPlanta.PosicaoPlanta_C|Getocupado _array_element))
            (Game|SpawnActorfromClass "Arvore_C" (Transformation|GetActorTransform _array_element) "Undefined" 0 0 2e+01 25.0 0)
            (Variables|/Game/Blueprints/PosicaoPlanta.PosicaoPlanta_C|Setocupado _array_element true)
            (goto _label Break))))
      (else
        (Default|Vitoria (Variables|Default|GetPlayerRef))))))

(event Custom|MensagensUsuario
  (bind _spawn (Variables|Default|Getspawn))
  (bind _outactors (Actor|GetAllActorsOfClass "Arvore_C"))
  (bind _output_get (Variables|Default|SetNumTreesAux (Utilities|Array|Length _outactors)))
  (Rendering|Components|TextRender|SetText (Variables|/Game/UI/HUD.HUD_C|GetMensagensConq (Variables|/Game/Blueprints/Player_BP.Player_BP_C|GetHUDRef (Variables|Default|GetPlayerRef))) (Utilities|Select :Index (- _output_get 1) :Option%200 (Variables|/Game/Blueprints/Spawner.Spawner_C|GetMSG1 _spawn) :Option%201 (Variables|/Game/Blueprints/Spawner.Spawner_C|GetMSG2 _spawn) :Option%202 (Variables|/Game/Blueprints/Spawner.Spawner_C|GetMSG3 _spawn) :Option%203 (Variables|/Game/Blueprints/Spawner.Spawner_C|GetMSG4 _spawn))))

(event EventBeginPlay
  (bind _asstatus_planta (Utilities|Casting|CastToStatusPlanta (UserInterface|GetWidget (Variables|Default|GetWidget))))
  (bind _output_get (Variables|Default|SetUI _asstatus_planta))
  (Variables|/Game/UI/StatusPlanta.StatusPlanta_C|Setarvore _output_get self)
  (CallFunction|AnimacaoFim)
  (Variables|Default|Setwater (Variables|Default|GetwaterLevel))
  (Variables|Default|Setfoton (Variables|Default|GetfotonLevel))
  (bind _asplayer_bp (Utilities|Casting|CastToPlayer_BP (Game|Player|GetPlayerPawn 0)))
  (Variables|Default|SetPlayerRef _asplayer_bp)
  (bind _returnvalue (Actor|GetActorOfClass "/Game/Blueprints/Spawner.Spawner_C"))
  (Variables|Default|Setspawn _returnvalue))

(event EventTick
  (params (DeltaSeconds :type Float%20%28single-precision%29))
  (CallFunction|Evolucao DeltaSeconds)
  (CallFunction|Derrota))

(fn ConstructionScript)

(fn UpdateUIPosition
  (Transformation|AddLocalOffset (Variables|Default|GetWidget) "0.000000,0.000000,64.000000" false false))