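; Agua is a 2D water projectile actor that moves by ProjectileMovement and splashes out when it reaches level bounds.
; Shortly after spawning it sets its first water sprite.
; When its Sphere overlaps an actor tagged "bounds", it destroys the sphere and stops moving.
; It then steps through two more sprites on timed delays as a simple impact animation before destroying itself.
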(event OnComponentBeginOverlap(Sphere)
  (params (OverlappedComponent :type Primitive%20Component%20Object%20Reference) (OtherActor :type Actor%20Object%20Reference) (OtherComp :type Primitive%20Component%20Object%20Reference) (OtherBodyIndex :type Integer) (bFromSweep :type Boolean) (SweepResult :type Hit%20Result%20Structure%20%28by%20ref%29))
  (if (Actor|ActorHasTag OtherActor "bounds")
    (Components|DestroyComponent (Variables|Default|GetSphere))
    (Components|Movement|StopMovementImmediately (Variables|Default|GetProjectileMovement))
    (Utilities|FlowControl|Delay 0.01)
    (Rendering|Components|Sprite|SetSprite (Variables|Default|GetPaperSprite) "/Game/Sprites/agua2_Sprite.agua2_Sprite")
    (Utilities|FlowControl|Delay 0.2)
    (Rendering|Components|Sprite|SetSprite (Variables|Default|GetPaperSprite) "/Game/Sprites/agua3_Sprite.agua3_Sprite")
    (Utilities|FlowControl|Delay 0.2)
    (Actor|DestroyActor)))

(event EventBeginPlay
  (Utilities|FlowControl|Delay 0.2)
  (Rendering|Components|Sprite|SetSprite (Variables|Default|GetPaperSprite) "/Game/Sprites/agua1_Sprite.agua1_Sprite"))

(fn ConstructionScript)